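; Prototype AI-controlled character that players can interact with to toggle its target, with visual debugging of its perception.
; Its action sets the instigator as the AIControllerTest's target, or clears any existing target.
; Each tick, an arrow is colored from Blackboard state: green for visible target, yellow for last known location, red otherwise.
; Tick also moves debug components to the eye viewpoint and controller focal point.
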(event EventBeginPlay
  (bind _self self)
  (bind _returnvalue (AI|GetAIController _self))
  (|CallParentFunction)
  (Development|SetHiddeninGame (Variables|Default|GetActionArrow) (not (Utilities|IsValid _returnvalue)) false)
  (Variables|Default|SetAIController _returnvalue))

(event EventTick
  (params (DeltaSeconds :type Float%20%28single-precision%29))
  (|CallParentFunction DeltaSeconds)
  (Utilities|FlowControl|Sequence
    (:then_0
      (|UpdateArrowColor))
    (:then_1
      (|DebugViewpoint))))

(event EventPerformAction
  (params (Instigator :type Pawn%20Object%20Reference))
  (bind _asaicontroller_test (Utilities|Casting|CastToAIControllerTest (Variables|Default|GetAIController)))
  (Default|SetCurrentTarget _asaicontroller_test (select (Utilities|IsValid (Default|GetCurrentTarget _asaicontroller_test)) 0 Instigator)))

(fn ConstructionScript
  (|CallParentFunction))

(fn GetActionPrimitive
  (return 0))

(fn GetActionText
  (return "Hello"))

(fn HasAction
  (return true))
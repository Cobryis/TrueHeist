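; Character Blueprint that handles AI target acquisition through its AIPerception component, which is active only when an AIController possesses it.
; Perception updates fill an empty blackboard Target with the first THCharacter found among currently perceived actors.
; The current Target is kept until a target perception update reports it is no longer sensed, which clears the key.
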(event OnPerceptionUpdated(AIPerception)
  (params (UpdatedActors :type Array%20of%20Actor%20Object%20References))
  (bind _returnvalue (AI|GetBlackboard 0))
  (Utilities|IsValid _returnvalue
    (:Is%20Valid
      (Utilities|IsValid (AI|Components|Blackboard|GetValueasObject _returnvalue (Utilities|Name|MakeLiteralName "Target"))
        (:Is%20Not%20Valid
          (bind _array_element (Utilities|Array|ForEachLoopwithBreak (Class|AIPerceptionComponent|GetCurrentlyPerceivedActors (Variables|Default|GetAIPerception)) :!label _label)
            (:LoopBody
              (bind _asthcharacter (Utilities|Casting|CastToTHCharacter _array_element))
              (AI|Components|Blackboard|SetValueasObject (AI|GetBlackboard 0) (Utilities|Name|MakeLiteralName "Target") _asthcharacter)
              (goto _label Break))))))))

(event OnTargetPerceptionUpdated(AIPerception)
  (params (Actor :type Actor%20Object%20Reference) (Stimulus :type AI%20Stimulus%20Structure))
  (bind _returnvalue (AI|GetBlackboard 0))
  (Utilities|IsValid _returnvalue
    (:Is%20Valid
      (if (== Actor (AI|Components|Blackboard|GetValueasObject _returnvalue (Utilities|Name|MakeLiteralName "Target")))
        (if (not (.bsuccessfullysensed Stimulus))
          (AI|Components|Blackboard|SetValueasObject (AI|GetBlackboard 0) (Utilities|Name|MakeLiteralName "Target") 0))))))

(event EventPossessed
  (params (NewController :type Controller%20Object%20Reference))
  (Components|Activation|SetActive (Variables|Default|GetAIPerception) (.bSuccess (Utilities|Casting|CastToAIController NewController)) false))

(fn ConstructionScript
  (|CallParentFunction))